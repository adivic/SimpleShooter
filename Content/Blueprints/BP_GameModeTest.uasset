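; BP_GameModeTest is a test game mode that scores kills and spawns zombie bots.
; When a non-player pawn dies, it adds score to that victim's own SPlayerState, not the killer's.
; SpawnNewBot runs the EQS_SpawnLocations query in random-best-25% mode and spawns BP_Zombie at the returned locations.
; On every fifth WaveCount, spawned zombies receive extra health, which is printed for debugging.
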(event `self.ReceiveBeginPlay`
  (add `self.OnActorKilled` (delegate `OnActorKilled_Event_0`)))

(event `OnActorKilled_Event_0` :!signature `self.OnActorKilled`
  (params (VictimActor :type "Actor Object Reference") (KillerActor :type "Actor Object Reference") (KillerController :type "Controller Object Reference"))
  (bind _aspawn (cast `Pawn` VictimActor))
  (if (not (`Pawn.IsPlayerControlled` _aspawn))
    (bind _assplayer_state (cast `SPlayerState` (`Pawn.PlayerState` _aspawn)))
    (`SPlayerState.AddScore` _assplayer_state 100.0)))

(event `self.SpawnNewBot`
  (bind _returnvalue (`EnvQueryManager.RunEQSQuery` "/Game/Blueprints/EQS_SpawnLocations.EQS_SpawnLocations" self "RandomBest25Pct"))
  (add `EnvQueryInstanceBlueprintWrapper.OnQueryFinishedEvent` _returnvalue (delegate `OnQueryFinishedEvent_Event_0`)))

(event `OnQueryFinishedEvent_Event_0`
  (params (QueryInstance :type "EnvQueryInstanceBlueprintWrapper Object Reference") (QueryStatus :type "EEnvQueryStatus Enum" :default "Processing"))
  (switch `EEnvQueryStatus` QueryStatus
    (:`Success`
      (bind _resultlocations (`EnvQueryInstanceBlueprintWrapper.GetQueryResultsAsLocations` QueryInstance))
      (for _array_element _resultlocations
        (bind _returnvalue (`|SpawnActorFromClass` "/Game/Blueprints/AI/BP_Zombie.BP_Zombie_C" (`KismetMathLibrary.MakeTransform` _array_element) "AdjustIfPossibleButDontSpawnIfColliding" "OverrideRootScale" null null))
        (if (== (mod (`self.WaveCount`) 5) 0)
          (bind _healthcomponent (`SCharacter.HealthComponent` _returnvalue))
          (bind _health (`SHealthComponent.Health` _healthcomponent))
          (`SHealthComponent.SetIncreaseHealt` _healthcomponent (+ _health 25.0))
          (`KismetSystemLibrary.PrintString` (`KismetStringLibrary.Conv_DoubleToString` _health) true false))))))

(fn `UserConstructionScript`)