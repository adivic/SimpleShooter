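; BP_Zombie is an AI enemy that runs the Zombie_BT behavior tree on BeginPlay and damages the player on contact.
; An Attack event briefly raises an IsAttack flag and prints a debug string.
; Damage comes separately from AttackCheck overlaps with BP_Player, without reading that flag, and only while the zombie's HealthComponent is not dead.
; A DoOnce limits damage to one hit until the player leaves the volume.
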(event `self.ReceiveBeginPlay`
  (`AIController.RunBehaviorTree` (`AIBlueprintHelperLibrary.GetAIController` self) "/Game/Blueprints/AI/Zombie_BT.Zombie_BT"))

(event `Attack`
  (set `self.IsAttack` true)
  (`KismetSystemLibrary.PrintString` "Attack")
  (`KismetSystemLibrary.Delay` 0.5)
  (set `self.IsAttack` false))

(event `self.AttackCheck.OnComponentBeginOverlap`
  (params (OverlappedComponent :type "PrimitiveComponent Object Reference") (OtherActor :type "Actor Object Reference") (OtherComp :type "PrimitiveComponent Object Reference") (OtherBodyIndex :type Integer) (bFromSweep :type Boolean) (SweepResult :type "HitResult Structure (by ref)"))
  (bind _asbp_player (cast `/Game/Blueprints/BP_Player` OtherActor))
  (`/Engine/EditorBlueprintResources/StandardMacros.DoOnce` false :!label _label
    (:`Completed`
      (if (not (`SHealthComponent.bIsDead` (`self.HealthComponent`)))
        (`GameplayStatics.ApplyDamage` _asbp_player 50.0)))))

(event `self.AttackCheck.OnComponentEndOverlap`
  (params (OverlappedComponent :type "PrimitiveComponent Object Reference") (OtherActor :type "Actor Object Reference") (OtherComp :type "PrimitiveComponent Object Reference") (OtherBodyIndex :type Integer))
  (cast `/Game/Blueprints/BP_Player` OtherActor)
  (goto _label :!via `Reset`))

(fn `UserConstructionScript`)